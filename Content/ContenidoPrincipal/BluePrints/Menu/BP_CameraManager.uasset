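; BP_CameraManager is a menu camera actor that moves its main camera between scene positions.
; On BeginPlay it snaps CameraMain to the PositionMain component's relative transform.
; CameraMovement restarts the Lerp timeline to blend the camera's relative location and rotation toward the given Scene component.
; Each update interpolates from the camera's current transform rather than a cached start, so motion compounds instead of following the alpha curve directly.
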(event `self.ReceiveBeginPlay`
  (bind _position_main (`self.Position_Main`))
  (`SceneComponent.K2_SetRelativeLocationAndRotation` (`self.CameraMain`) (`SceneComponent.RelativeLocation` _position_main) (`SceneComponent.RelativeRotation` _position_main) false false))

(event `CameraMovement`
  (params (Scene :type "SceneComponent Object Reference"))
  (bind _cameramain (`self.CameraMain`))
  (bind (_direction _alpha) (`Timeline|lerp` :!via `PlayFromStart`)
    (:`Update`
      (`SceneComponent.K2_SetRelativeLocationAndRotation` (`self.CameraMain`) (`KismetMathLibrary.VLerp` (`SceneComponent.RelativeLocation` _cameramain) (`SceneComponent.RelativeLocation` Scene) _alpha) (`KismetMathLibrary.RLerp` (`SceneComponent.RelativeRotation` _cameramain) (`SceneComponent.RelativeRotation` Scene) _alpha) false false))))

(fn `UserConstructionScript`)