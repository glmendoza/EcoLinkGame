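; GM_LevelPlaza_1 is the game mode for a plaza level, tying waste cleanup progress to NPC activation and level completion.
; On BeginPlay it caches the BP_SetNPC actor found in the level.
; It extends the parent's waste calculation, using the resulting percentage to activate two NPC stages at rising thresholds.
; When that percentage reaches one hundred, it flags the level as clean.
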(event `self.ReceiveBeginPlay`
  (`parent.ReceiveBeginPlay`)
  (bind _returnvalue (`GameplayStatics.GetActorOfClass` "/Game/ContenidoPrincipal/BluePrints/NPCs/NPCBaseTest/BP_SetNPC.BP_SetNPC_C"))
  (set `self.Set NPC ref` _returnvalue))

(event `self.CalculateRemainingWaste`
  (params (Cantidad :type Integer))
  (`parent.CalculateRemainingWaste` Cantidad)
  (`self.Spawn NPCs`)
  (if (>= (`self.RemainingPorcentage`) 100.0)
    (set `self.LevelClean` true)))

(event `Spawn NPCs`
  (if (>= (`self.RemainingPorcentage`) 20.0)
    (`/Game/ContenidoPrincipal/BluePrints/NPCs/NPCBaseTest/BP_SetNPC.ACtivate NPC 1` (`self.Set NPC ref`))
    (if (>= (`self.RemainingPorcentage`) 60.0)
      (`/Game/ContenidoPrincipal/BluePrints/NPCs/NPCBaseTest/BP_SetNPC.Activate NPC 2` (`self.Set NPC ref`)))))

(fn `UserConstructionScript`
  (`parent.UserConstructionScript`))