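; Base game mode for a waste cleanup level that opens a tutorial widget in UI-only input and tracks how clean the level is.
; At BeginPlay it counts all BP_Residuo actors and caches the player character.
; CalculateRemainingWaste updates the HUD clean percentage, flags the level clean at completion and calls SpawnNPC.
; SpawnNPC keeps a single random-waste-type NPC once a small progress threshold is reached; AddScore is an empty stub.
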(event `self.ReceiveBeginPlay`
  (bind _returnvalue (`GameplayStatics.GetPlayerController` 0))
  (`self.EnableInput` _returnvalue)
  (`self.Set Variables`)
  (bind _returnvalue_2 (`|CreateWidget` "/Game/ContenidoPrincipal/BluePrints/UI/Tutorials/WBP_Tutorials_Base.WBP_Tutorials_Base_C" _returnvalue))
  (`UserWidget.AddToViewport` _returnvalue_2 1)
  (set `PlayerController.bShowMouseCursor` true _returnvalue)
  (`WidgetBlueprintLibrary.SetInputMode_UIOnlyEx` _returnvalue null))

(event `Set Variables`
  ;[1 0 0] Inicializa las variables
  (bind _outactors (`GameplayStatics.GetAllActorsOfClass` "/Game/ContenidoPrincipal/BluePrints/LevelObjects/BP_Residuo.BP_Residuo_C"))
  (bind _output_get (set `self.Residuos` _outactors))
  (bind _output_get_2 (set `self.TotalWaste` (`KismetMathLibrary.Conv_IntToDouble` (`KismetArrayLibrary.Array_Length` _output_get))))
  (set `self.RemainingWaste` _output_get_2)
  (bind _astpc_principal (cast `/Game/ContenidoPrincipal/BluePrints/Character/TPC_Principal` (`GameplayStatics.GetPlayerCharacter` 0)))
  (set `self.PlayerRef` _astpc_principal))

(event `CalculateRemainingWaste`
  ;[1 0.3333 0] Calcula el procentage de desechos recolectado en el nivel
  (set `self.RemainingWaste` (- (`self.RemainingWaste`) 1.0))
  (bind _output_get (set `self.RemainingPorcentage` (* (- 1.0 (/ (`self.RemainingWaste`) (`self.TotalWaste`))) 100.0)))
  (`/Game/ContenidoPrincipal/BluePrints/UI/PlayerHUD/WBP_CleanPercentage.SetTextPercentage` (`/Game/ContenidoPrincipal/BluePrints/UI/PlayerHUD/WBP_PlayerHUD.WBP_CleanPercentage` (`/Game/ContenidoPrincipal/BluePrints/Character/TPC_Principal.PlayerHUD Ref` (`self.PlayerRef`))) _output_get)
  (`self.SpawnNPC`)
  (if (>= (`self.RemainingPorcentage`) 100.0)
    (set `self.LevelClean` true)))

(event `AddScore`
  (params (`Score to Add` :type Integer)))

(event `SpawnNPC`
  (if (>= (`self.RemainingPorcentage`) 5.0)
    (`/Engine/EditorBlueprintResources/StandardMacros.IsValid` (`self.NPC Ref`)
      (:`Is Not Valid`
        (bind _returnvalue (`|SpawnActorFromClass` "/Game/ContenidoPrincipal/BluePrints/NPCs/BP_NPC_1.BP_NPC_1_C" (`KismetMathLibrary.Conv_VectorToTransform` (`self.SpawnPosition`)) "Undefined" "OverrideRootScale" null (cast `/Game/ContenidoPrincipal/BluePrints/Interfaces/E_WasteType` (`KismetMathLibrary.Conv_IntToByte` (`KismetMathLibrary.RandomIntegerInRange` 0 4))) null))
        (set `self.NPC Ref` _returnvalue)
        (`KismetSystemLibrary.PrintString` "NPC creado" true true (struct :`R` 1.0 :`B` 1.0 :`A` 1.0) 5.0)))))

(fn `UserConstructionScript`)