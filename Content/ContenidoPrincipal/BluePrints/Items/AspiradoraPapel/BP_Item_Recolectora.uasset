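; BP_Item_Recolectora is a vacuum-style collector item that picks up waste matching its configured material type.
; Primary use starts a looping timer and attaches an air vortex Niagara effect; stopping clears both.
; Each timer tick sphere-traces forward from below the player character's center and calls PickWaste on a hit BP_Residuo whose WasteType matches MaterialToRecolect.
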(event `self.UseItemPrimary`
  (if (not (`self.IsCollecting`))
    (set `self.IsCollecting` true)
    (`KismetSystemLibrary.K2_SetTimer` null "CastShape" 0.1 true)
    (bind _returnvalue (`NiagaraFunctionLibrary.SpawnSystemAttached` "/Game/ContenidoPrincipal/BluePrints/Items/AspiradoraPapel/NS_AirVortex.NS_AirVortex" (`self.vfx`) "None" (0.0 0.0 0.0) (struct) "KeepRelativeOffset"))
    (set `self.FX` _returnvalue)))

(event `self.StopItem`
  (if (`self.IsCollecting`)
    (set `self.IsCollecting` false)
    (`KismetSystemLibrary.K2_ClearTimer` null "CastShape")
    (`ActorComponent.K2_DestroyComponent` (`self.Fx`))))

(event `CastShape`
  (bind _returnvalue (`GameplayStatics.GetPlayerCharacter` 0))
  (bind _returnvalue_2 (- (`self.K2_GetActorLocation` _returnvalue) (0.0 0.0 50.0)))
  (bind _outhit (`KismetSystemLibrary.SphereTraceSingle` :`Start` _returnvalue_2 :`End` (+ _returnvalue_2 (* (`self.GetActorForwardVector` _returnvalue) 400.0)) :`Radius` 100.0 :`TraceChannel` "TraceTypeQuery1" :`DrawTime` 1.0))
  (bind _asbp_residuo (cast `/Game/ContenidoPrincipal/BluePrints/LevelObjects/BP_Residuo` (`.HitActor` (`GameplayStatics.BreakHitResult` _outhit))))
  (`/Engine/EditorBlueprintResources/StandardMacros.IsValid` _asbp_residuo
    (:`Is Valid`
      (if (`|EnumEquality` (`/Game/ContenidoPrincipal/BluePrints/LevelObjects/BP_Residuo.WasteType` _asbp_residuo) (`self.MaterialToRecolect`))
        (`/Game/ContenidoPrincipal/BluePrints/LevelObjects/BP_Residuo.PickWaste` _asbp_residuo)))))

(fn `UserConstructionScript`
  (`parent.UserConstructionScript`))