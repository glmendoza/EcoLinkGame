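; BP_Guantes is a gloves item whose primary use lets the player pick up one type of waste in front of them.
; UseItemPrimary plays a montage on the player and waits a third of its length before calling CastShape.
; CastShape runs a box trace on the Visibility channel just ahead of the player character, calling PickWaste on a hit BP_Residuo of the matching WasteType.
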(event `self.UseItemPrimary`
  (bind _returnvalue (`Character.PlayAnimMontage` (`self.Player Ref`) "/Game/ContenidoPrincipal/BluePrints/Character/Player/PlayerModel1/Animations/Drop_Montage.Drop_Montage" 1.0 "None"))
  (`KismetSystemLibrary.Delay` (/ _returnvalue 3.0))
  (`self.Cast shape`))

(event `Cast shape`
  (bind _returnvalue (`GameplayStatics.GetPlayerCharacter` 0))
  (bind _returnvalue_2 (`self.GetActorForwardVector` _returnvalue))
  (bind _returnvalue_3 (+ (- (`self.K2_GetActorLocation` _returnvalue) (0.0 0.0 10.0)) (* _returnvalue_2 50.0)))
  (bind _outhit (`KismetSystemLibrary.BoxTraceSingle` :`Start` _returnvalue_3 :`End` _returnvalue_3 :`HalfSize` (50.0 50.0 90.0) :`Orientation` (`KismetMathLibrary.Conv_VectorToRotator` _returnvalue_2) :`TraceChannel` "TraceTypeQuery1" :`DrawTime` 0.2))
  (bind _asbp_residuo (cast `/Game/ContenidoPrincipal/BluePrints/LevelObjects/BP_Residuo` (`.HitActor` (`GameplayStatics.BreakHitResult` _outhit))))
  (if (`|EnumEquality` (`/Game/ContenidoPrincipal/BluePrints/LevelObjects/BP_Residuo.WasteType` _asbp_residuo) "NewEnumerator1")
    (`/Game/ContenidoPrincipal/BluePrints/LevelObjects/BP_Residuo.PickWaste` _asbp_residuo)))

(fn `UserConstructionScript`
  (`parent.UserConstructionScript`))