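; BP_RecolectorCigarro is a usable item, apparently a stick, for picking up cigars in the world.
; Primary use runs CastShape, then plays the UseStick montage on the player.
; CastShape does a stationary Visibility box trace just in front of player 0 and calls PickCigar on a hit BP_Cigar.
; The trace's debug drawing is left on.
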(event `self.UseItemPrimary`
  (`self.Cast Shape`)
  (`Character.PlayAnimMontage` (`self.Player Ref`) "/Game/ContenidoPrincipal/Meshes/Player/PlayerModel1/Animations/UseStick_Montage.UseStick_Montage" 1.0 "None"))

(event `Cast Shape`
  (bind _returnvalue (`GameplayStatics.GetPlayerCharacter` 0))
  (bind _returnvalue_2 (`self.GetActorForwardVector` _returnvalue))
  (bind _returnvalue_3 (+ (- (`self.K2_GetActorLocation` _returnvalue) (0.0 0.0 10.0)) (* _returnvalue_2 50.0)))
  (bind _outhit (`KismetSystemLibrary.BoxTraceSingle` :`Start` _returnvalue_3 :`End` _returnvalue_3 :`HalfSize` (50.0 50.0 90.0) :`Orientation` (`KismetMathLibrary.Conv_VectorToRotator` _returnvalue_2) :`TraceChannel` "TraceTypeQuery1" :`DrawDebugType` "ForDuration" :`DrawTime` 1.0))
  (bind _asbp_cigar (cast `/Game/ContenidoPrincipal/BluePrints/LevelObjects/BP_Cigar` (`.HitActor` (`GameplayStatics.BreakHitResult` _outhit))))
  (`/Engine/EditorBlueprintResources/StandardMacros.IsValid` _asbp_cigar
    (:`Is Valid`
      (`/Game/ContenidoPrincipal/BluePrints/LevelObjects/BP_Cigar.PickCigar` _asbp_cigar))))

(fn `UserConstructionScript`
  (`parent.UserConstructionScript`))