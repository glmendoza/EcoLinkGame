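; Base item actor the player picks up into their inventory, with empty primary, secondary and stop use events.
; Sphere overlap checks inventory space, shows the interact prompt and switches the mesh's custom-depth stencil.
; Interact stores the item, disables collision, hides the mesh and opens any tutorial widget in UI-only input.
; Construction sets sphere radius and optional tint; helper functions attach or detach left/right meshes on player sockets.
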(event `self.ReceiveBeginPlay`
  ;[1 1 1] Inizializa la variable del jugador
  (bind _astpc_principal (cast `/Game/ContenidoPrincipal/BluePrints/Character/TPC_Principal` (`GameplayStatics.GetPlayerCharacter` 0)))
  (set `self.Player Ref` _astpc_principal))

(event `UseItemPrimary`
  ;[1 1 1] Activa el funcionamiento del item
)

(event `UseItemSecundary`
  ;[1 1 1] Activa el funcionamiento del item
)

(event `StopItem`
  ;[1 1 1] Activa el funcionamiento del item
)

(event `/Game/ContenidoPrincipal/BluePrints/Interfaces/BPI_Interface.Interact`
  ;[1 1 1] Evento de interaccion
  (if (`self.Can Interact`)
    (`/Game/ContenidoPrincipal/BluePrints/Character/TPC_Principal.AddItemsToInventory` (`self.Player Ref`) self)
    (`self.SetActorEnableCollision` false)
    (`SceneComponent.SetVisibility` (`self.Main Item`) false false)
    (`/Game/ContenidoPrincipal/BluePrints/Character/TPC_Principal.HideInteractUI` (`self.Player Ref`))
    (`self.WidgetTut`)))

(event `WidgetTut`
  (bind _returnvalue (`GameplayStatics.GetPlayerController` 0))
  (bind _widget (`self.Widget`))
  ;[1 1 1] Si el item tiene un widget de tutorial, este parecera en pantalla
  (if (`KismetSystemLibrary.IsValidClass` _widget)
    (bind _returnvalue_2 (`|CreateWidget` _widget _returnvalue))
    (`UserWidget.AddToViewport` _returnvalue_2 1)
    (set `PlayerController.bShowMouseCursor` true _returnvalue)
    (`WidgetBlueprintLibrary.SetInputMode_UIOnlyEx` _returnvalue null)))

(event `self.SphereColl.OnComponentBeginOverlap`
  (params (OverlappedComponent :type "PrimitiveComponent Object Reference") (OtherActor :type "Actor Object Reference") (OtherComp :type "PrimitiveComponent Object Reference") (OtherBodyIndex :type Integer) (bFromSweep :type Boolean) (SweepResult :type "HitResult Structure (by ref)"))
  (bind _player_ref (`self.Player Ref`))
  (if (`self.ActorHasTag` OtherActor "Player")
    (set `self.Can Interact` (< (`KismetArrayLibrary.Array_Length` (`/Game/ContenidoPrincipal/BluePrints/Character/TPC_Principal.InventoryForItems` _player_ref)) (`/Game/ContenidoPrincipal/BluePrints/Character/TPC_Principal.MaxInventorySize` _player_ref)))
    (`PrimitiveComponent.SetCustomDepthStencilValue` (`self.Main Item`) 3)
    (`/Game/ContenidoPrincipal/BluePrints/Character/TPC_Principal.ShowInteractUI` (`self.Player Ref`) "E - Equipar")))

(event `self.SphereColl.OnComponentEndOverlap`
  (params (OverlappedComponent :type "PrimitiveComponent Object Reference") (OtherActor :type "Actor Object Reference") (OtherComp :type "PrimitiveComponent Object Reference") (OtherBodyIndex :type Integer))
  (if (`self.ActorHasTag` OtherActor "Player")
    (`PrimitiveComponent.SetCustomDepthStencilValue` (`self.Main Item`) 2)
    (`/Game/ContenidoPrincipal/BluePrints/Character/TPC_Principal.HideInteractUI` (`self.Player Ref`))))

(fn `EquipDoubleItem`
  (bind _item_izq (`self.Item Izq`))
  (bind _item_der (`self.Item Der`))
  (bind _mesh (`Character.Mesh` (`self.Player Ref`)))
  (`|ExecutionSequence`
    (:`then_0`
      (`/Engine/EditorBlueprintResources/StandardMacros.IsValid` _item_izq
        (:`Is Valid`
          (`SceneComponent.SetVisibility` _item_izq true false)
          (`SceneComponent.K2_AttachToComponent` _item_izq _mesh "Item Izq" "SnapToTarget" "SnapToTarget" "KeepRelative" true))))
    (:`then_1`
      (`/Engine/EditorBlueprintResources/StandardMacros.IsValid` _item_der
        (:`Is Valid`
          (`SceneComponent.SetVisibility` _item_der true false)
          (`SceneComponent.K2_AttachToComponent` _item_der _mesh "Item Der" "SnapToTarget" "SnapToTarget" "KeepRelative" true))))))

(fn `RemoveDoubleItem`
  (bind _item_izq (`self.Item Izq`))
  (bind _item_der (`self.Item Der`))
  (`|ExecutionSequence`
    (:`then_0`
      (`/Engine/EditorBlueprintResources/StandardMacros.IsValid` _item_izq
        (:`Is Valid`
          (`SceneComponent.SetVisibility` _item_izq false false)
          (`SceneComponent.K2_DetachFromComponent` _item_izq "KeepRelative" "KeepRelative" "KeepRelative" true))))
    (:`then_1`
      (`/Engine/EditorBlueprintResources/StandardMacros.IsValid` _item_der
        (:`Is Valid`
          (`SceneComponent.SetVisibility` _item_der false false)
          (`SceneComponent.K2_DetachFromComponent` _item_der "KeepRelative" "KeepRelative" "KeepRelative" true))))))

(fn `UserConstructionScript`
  (`SphereComponent.SetSphereRadius` (`self.SphereColl`) (`self.In Sphere Radius`) true)
  (if (not (`self.UseText`))
    (bind _returnvalue (`PrimitiveComponent.CreateDynamicMaterialInstance` (`self.Main Item`) 0 "/Game/ContenidoPrincipal/Materials/M_Test_Color.M_Test_Color" "None"))
    (`MaterialInstanceDynamic.SetVectorParameterValue` _returnvalue "Color" (`self.Color`))))