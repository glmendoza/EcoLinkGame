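; BP_SetNPC is a helper Blueprint that switches referenced NPCs into walking movement.
; ActivateNPC1 maps an index from 0 to 4 to one of five stored NPC references and passes it to SetNPC.
; SetNPC sets that character's movement mode to Walking through a DoOnce node inside the function.
; The event graph and construction script are empty, so activation relies on calls to these functions.
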(fn `ActivateNPC1`
  (params (Index :type Integer))
  (switch `int` Index
    (:`0`
      (`self.SetNPC` (`self.NPC Ref 1`)))
    (:`1`
      (`self.SetNPC` (`self.NPC Ref 2`)))
    (:`2`
      (`self.SetNPC` (`self.NPC Ref 3`)))
    (:`3`
      (`self.SetNPC` (`self.NPC Ref 4`)))
    (:`4`
      (`self.SetNPC` (`self.NPC Ref 5`)))))

(fn `SetNPC`
  (params (NPC :type "Character Object Reference"))
  (`/Engine/EditorBlueprintResources/StandardMacros.DoOnce` false
    (:`Completed`
      (`CharacterMovementComponent.SetMovementMode` (`Character.CharacterMovement` NPC) "MOVE_Walking" 0))))

(fn `UserConstructionScript`)