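; BP_CrowdManager is a placement actor that lays out a crowd as a grid of child actors.
; Its construction script loops over Filas and Columnas, adding one child actor component per cell, spaced by Espaciado and jittered randomly by Offset in X and Y.
; Components use manual attachment, with positions offset from the manager's location, a fixed height and the manager's rotation, which does not rotate the grid.
; The event graph is empty.
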(fn `UserConstructionScript`
  (bind (_returnvalue_x _returnvalue_y) (`KismetMathLibrary.BreakVector` (`self.K2_GetActorLocation`)))
  (bind _espaciado (`self.Espaciado`))
  (bind _offset (`self.Offset`))
  (bind _returnvalue (`KismetMathLibrary.RandomFloatInRange` (* _offset -1.0) _offset))
  (for _index (range (`self.Filas`))
    (for _index_2 (range (`self.Columnas`))
      (`AddComponent|NODE_AddChildActorComponent-0` :`bManualAttachment` true :`RelativeTransform` (`KismetMathLibrary.MakeTransform` (`KismetMathLibrary.MakeVector` (+ (+ (* _index_2 _espaciado) _returnvalue) _returnvalue_x) (+ (+ (* _index _espaciado) _returnvalue) _returnvalue_y) 50.0) (`self.K2_GetActorRotation`))))))