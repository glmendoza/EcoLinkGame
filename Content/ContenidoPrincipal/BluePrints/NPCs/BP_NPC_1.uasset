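; NPC character that drops a random type of waste and can be talked to by the player for score.
; Overlapping the player while its waste exists shows a talk prompt, turns the NPC and sets a blackboard flag.
; Interacting sets another flag, awards points and speeds the NPC up.
; Separate events find the container matching the waste type, attach the waste to a hand socket, and later destroy it and restore walk speed.
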(event `self.ReceiveBeginPlay`
  (bind _outactors (`GameplayStatics.GetAllActorsOfClass` "/Game/ContenidoPrincipal/BluePrints/LevelObjects/BP_Container.BP_Container_C"))
  (set `self.Containers` _outactors)
  (bind _astpgame_mode_base (cast `/Game/ContenidoPrincipal/BluePrints/GameModes/TPGameMode_Base` (`GameplayStatics.GetGameMode`)))
  (set `self.GameModeRef` _astpgame_mode_base)
  (bind _astpc_principal (cast `/Game/ContenidoPrincipal/BluePrints/Character/TPC_Principal` (`GameplayStatics.GetPlayerCharacter` 0)))
  (set `self.Player Ref` _astpc_principal)
  (bind _returnvalue (`GameplayStatics.GetActorOfClass` "/Game/ContenidoPrincipal/BluePrints/NPCs/BP_NPCSpawner.BP_NPCSpawner_C"))
  (`/Engine/EditorBlueprintResources/StandardMacros.IsValid` _returnvalue
    (:`Is Valid`
      (set `self.FinalPosition` (`self.K2_GetActorLocation` _returnvalue)))))

(event `/Game/ContenidoPrincipal/BluePrints/Interfaces/BPI_Interface.Interact`
  (bind _returnvalue (`AIBlueprintHelperLibrary.GetBlackboard` null))
  ;[1 1 1] Comment
  (`/Engine/EditorBlueprintResources/StandardMacros.IsValid` (`self.ActualWaste`)
    (:`Is Valid`
      (if (not (`BlackboardComponent.GetValueAsBool` _returnvalue "PlayerInteracted"))
        (`BlackboardComponent.SetValueAsBool` _returnvalue "PlayerInteracted" true)
        (set `self.Inetractuado` true)
        (`KismetSystemLibrary.PrintString` "Interaccion con exito")
        (`/Game/ContenidoPrincipal/BluePrints/Character/TPC_Principal.HideInteractUI` (`self.Player Ref`))
        (`/Game/ContenidoPrincipal/BluePrints/GameModes/TPGameMode_Base.AddScore` (`self.GameModeRef`) 1000)
        (set `CharacterMovementComponent.MaxWalkSpeed` 500.0 (`self.CharacterMovement`))))))

(event `DropTrash`
  ;[1 1 1] Comment
  (`/Engine/EditorBlueprintResources/StandardMacros.DoOnce` false
    (:`Completed`
      (bind _returnvalue (`|SpawnActorFromClass` "/Game/ContenidoPrincipal/BluePrints/LevelObjects/BP_Residuo.BP_Residuo_C" (`KismetMathLibrary.Conv_VectorToTransform` (- (`self.K2_GetActorLocation`) (0.0 0.0 86.0))) "Undefined" "OverrideRootScale" null (cast `/Game/ContenidoPrincipal/BluePrints/Interfaces/E_WasteType` (`KismetMathLibrary.Conv_IntToByte` (`KismetMathLibrary.RandomIntegerInRange` 0 4))) false null))
      (set `self.ActualWaste` _returnvalue))))

(event `FindContainer`
  ;[1 1 1] Comment
  (`/Engine/EditorBlueprintResources/StandardMacros.DoOnce` false
    (:`Completed`
      (`self.AttachDesecho`)
      (for _array_element (`self.Containers`)
        (if (`|EnumEquality` (`/Game/ContenidoPrincipal/BluePrints/LevelObjects/BP_Container.WasteType` _array_element) (`/Game/ContenidoPrincipal/BluePrints/LevelObjects/BP_Residuo.WasteType` (`self.ActualWaste`)))
          (set `self.TargetContainer` _array_element))))))

(event `AttachDesecho`
  ;[1 1 1] Comment
  (`self.K2_AttachToComponent` (`self.ActualWaste`) (`self.Mesh`) "ItemSocket" "SnapToTarget" "SnapToTarget" "KeepRelative" true))

(event `self.Interact_Coll.OnComponentBeginOverlap`
  (params (OverlappedComponent :type "PrimitiveComponent Object Reference") (OtherActor :type "Actor Object Reference") (OtherComp :type "PrimitiveComponent Object Reference") (OtherBodyIndex :type Integer) (bFromSweep :type Boolean) (SweepResult :type "HitResult Structure (by ref)"))
  (bind (_returnvalue_roll _returnvalue_pitch _returnvalue_yaw) (`KismetMathLibrary.BreakRotator` (`KismetMathLibrary.FindLookAtRotation` (`self.K2_GetActorLocation`) (`self.K2_GetActorLocation` (`self.Player Ref`)))))
  (if (`self.ActorHasTag` OtherActor "Player")
    (`/Engine/EditorBlueprintResources/StandardMacros.IsValid` (`self.ActualWaste`)
      (:`Is Valid`
        (if (not (`self.Inetractuado`))
          (`BlackboardComponent.SetValueAsInt` (`AIBlueprintHelperLibrary.GetBlackboard` null) "Istalking" 1)
          (`self.K2_SetActorRotation` (`KismetMathLibrary.MakeRotator` 0.0 0.0 _returnvalue_yaw))
          (`/Game/ContenidoPrincipal/BluePrints/Character/TPC_Principal.ShowInteractUI` (`self.Player Ref`) "E - Hablar"))))))

(event `DetachDesecho`
  (bind _actualwaste (`self.ActualWaste`))
  ;[1 1 1] Comment
  (`self.K2_DetachFromActor` _actualwaste "KeepRelative" "KeepRelative" "KeepRelative")
  (`KismetSystemLibrary.Delay` 0.2)
  (`self.K2_DestroyActor` _actualwaste)
  (set `CharacterMovementComponent.MaxWalkSpeed` 200.0 (`self.CharacterMovement`)))

(event `self.Interact_Coll.OnComponentEndOverlap`
  (params (OverlappedComponent :type "PrimitiveComponent Object Reference") (OtherActor :type "Actor Object Reference") (OtherComp :type "PrimitiveComponent Object Reference") (OtherBodyIndex :type Integer))
  (if (`self.ActorHasTag` OtherActor "Player")
    (`BlackboardComponent.SetValueAsInt` (`AIBlueprintHelperLibrary.GetBlackboard` null) "Istalking" 0)
    (`/Game/ContenidoPrincipal/BluePrints/Character/TPC_Principal.HideInteractUI` (`self.Player Ref`))))

(fn `UserConstructionScript`)