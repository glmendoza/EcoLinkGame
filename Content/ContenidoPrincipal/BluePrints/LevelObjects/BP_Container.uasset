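; BP_Container is a waste-sorting bin where the player deposits collected waste of one configured type for points.
; The construction script sets the label and bin material from WasteType.
; A box overlap shows the deposit prompt and switches custom-depth stencil highlighting.
; Interact adds score per unit, updates the game mode's remaining waste, zeroes that type in the player's material map and refreshes the HUD.
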(event `self.ReceiveBeginPlay`
  (bind _astpc_principal (cast `/Game/ContenidoPrincipal/BluePrints/Character/TPC_Principal` (`GameplayStatics.GetPlayerCharacter` 0)))
  (set `self.PlayerRef` _astpc_principal)
  (bind _astpgame_mode_base (cast `/Game/ContenidoPrincipal/BluePrints/GameModes/TPGameMode_Base` (`GameplayStatics.GetGameMode`)))
  (set `self.GameModeRef` _astpgame_mode_base))

(event `/Game/ContenidoPrincipal/BluePrints/Interfaces/BPI_Interface.Interact`
  (bind _playerref (`self.PlayerRef`))
  (bind _gamemoderef (`self.GameModeRef`))
  (bind _returnvalue (`|GetEnumeratorNameAsString` (`self.WasteType`)))
  (bind _materialstocollect (`/Game/ContenidoPrincipal/BluePrints/Character/TPC_Principal.MaterialsToCollect` (`self.PlayerRef`)))
  (bind _value (`BlueprintMapLibrary.Map_Find` _materialstocollect _returnvalue))
  ;[1 1 1] Elimina los desechos que tenga el jugador y aumenta el puntaje segun la cantidad que tenga
  (if (>= (`BlueprintMapLibrary.Map_Find` _materialstocollect _returnvalue) 1)
    (`/Game/ContenidoPrincipal/BluePrints/GameModes/TPGameMode_Base.AddScore` _gamemoderef (* _value (`KismetMathLibrary.RandomIntegerInRange` 100 100)))
    (`/Game/ContenidoPrincipal/BluePrints/GameModes/TPGameMode_Base.CalculateRemainingWaste` _gamemoderef _value)
    (`BlueprintMapLibrary.Map_Add` _materialstocollect (`|GetEnumeratorNameAsString` (`self.WasteType`)) (- _value _value))
    (`/Game/ContenidoPrincipal/BluePrints/Character/TPC_Principal.SetMaterialHUD` _playerref)
    (`/Game/ContenidoPrincipal/BluePrints/Character/TPC_Principal.HideInteractUI` _playerref)))

(event `self.BoxColl.OnComponentBeginOverlap`
  (params (OverlappedComponent :type "PrimitiveComponent Object Reference") (OtherActor :type "Actor Object Reference") (OtherComp :type "PrimitiveComponent Object Reference") (OtherBodyIndex :type Integer) (bFromSweep :type Boolean) (SweepResult :type "HitResult Structure (by ref)"))
  (if (`self.ActorHasTag` OtherActor "Player")
    (`PrimitiveComponent.SetCustomDepthStencilValue` (`self.Contenedor`) 2)
    (`/Game/ContenidoPrincipal/BluePrints/Character/TPC_Principal.ShowInteractUI` (`self.PlayerRef`) "E - Depositar Residuos")))

(event `self.BoxColl.OnComponentEndOverlap`
  (params (OverlappedComponent :type "PrimitiveComponent Object Reference") (OtherActor :type "Actor Object Reference") (OtherComp :type "PrimitiveComponent Object Reference") (OtherBodyIndex :type Integer))
  (if (`self.ActorHasTag` OtherActor "Player")
    (`PrimitiveComponent.SetCustomDepthStencilValue` (`self.Contenedor`) 1)
    (`/Game/ContenidoPrincipal/BluePrints/Character/TPC_Principal.HideInteractUI` (`self.PlayerRef`))))

(fn `UserConstructionScript`
  (bind _contenedor (`self.Contenedor`))
  (`TextRenderComponent.K2_SetText` (`self.TextRender`) (`self.Text`))
  (switch `/Game/ContenidoPrincipal/BluePrints/Interfaces/E_WasteType` (`self.WasteType`)
    (:`NewEnumerator0`
      (`PrimitiveComponent.SetMaterial` _contenedor 0 "/Game/ContenidoPrincipal/Meshes/ContenedorMadera/Mi_ContenedorPlastic.Mi_ContenedorPlastic"))
    (:`NewEnumerator1`
      (`PrimitiveComponent.SetMaterial` _contenedor 0 "/Game/ContenidoPrincipal/Meshes/ContenedorMadera/Mi_Contenedor__Glass.Mi_Contenedor__Glass"))
    (:`NewEnumerator2`
      (`PrimitiveComponent.SetMaterial` _contenedor 0 "/Game/ContenidoPrincipal/Meshes/ContenedorMadera/Mi_Contenedor_Paper.Mi_Contenedor_Paper"))
    (:`NewEnumerator3`
      (`PrimitiveComponent.SetMaterial` _contenedor 0 "/Game/ContenidoPrincipal/Meshes/ContenedorMadera/Mi_Contenedor__Organic.Mi_Contenedor__Organic"))
    (:`NewEnumerator4`
      (`PrimitiveComponent.SetMaterial` _contenedor 0 "/Game/ContenidoPrincipal/Meshes/ContenedorMadera/Mi_Contenedor__Others.Mi_Contenedor__Others"))))