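; BP_Macetas is an interactable plant pot that the player can plant once.
; A Box overlap with the tagged player toggles an interact icon and the player's planting prompt.
; Interact locks the pot, fires a star burst, reveals the plant mesh and increments MacetasPlantadas on the game mode.
; The construction script tints the icon from ColorIcon and sets up the burst's Niagara parameters.
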(event `self.ReceiveBeginPlay`
  (bind _astpc_principal (cast `/Game/ContenidoPrincipal/BluePrints/Character/TPC_Principal` (`GameplayStatics.GetPlayerCharacter` 0)))
  (set `self.PlayerRef` _astpc_principal)
  (bind _astpgame_mode_base (cast `/Game/ContenidoPrincipal/BluePrints/GameModes/TPGameMode_Base` (`GameplayStatics.GetGameMode`)))
  (set `self.GameModeRef` _astpgame_mode_base))

(event `/Game/ContenidoPrincipal/BluePrints/Interfaces/BPI_Interface.Interact`
  (bind _gamemoderef (`self.GameModeRef`))
  (if (not (`self.Interacted`))
    (set `self.Interacted` true)
    (`ActorComponent.Activate` (`self.NS_BurstStars`) true)
    (`SceneComponent.SetVisibility` (`self.Interact Icon`) false false)
    (`SceneComponent.SetVisibility` (`self.SM_Maceta_SM_Maceta_Planta`) true false)
    (`/Game/ContenidoPrincipal/BluePrints/Character/TPC_Principal.HideInteractUI` (`self.PlayerRef`))
    (bind _result (`/Engine/EditorBlueprintResources/StandardMacros.IncrementInt` (`/Game/ContenidoPrincipal/BluePrints/GameModes/TPGameMode_Base.MacetasPlantadas` _gamemoderef))
      (:`  `
        (set `/Game/ContenidoPrincipal/BluePrints/GameModes/TPGameMode_Base.MacetasPlantadas` _result _gamemoderef)))))

(event `self.Box.OnComponentBeginOverlap`
  (params (OverlappedComponent :type "PrimitiveComponent Object Reference") (OtherActor :type "Actor Object Reference") (OtherComp :type "PrimitiveComponent Object Reference") (OtherBodyIndex :type Integer) (bFromSweep :type Boolean) (SweepResult :type "HitResult Structure (by ref)"))
  (if (`self.ActorHasTag` OtherActor "Player")
    (if (not (`self.Interacted`))
      (`/Game/ContenidoPrincipal/BluePrints/Character/TPC_Principal.ShowInteractUI` (`self.PlayerRef`) "E - Plantar")
      (`SceneComponent.SetVisibility` (`self.Interact Icon`) true false))))

(event `self.Box.OnComponentEndOverlap`
  (params (OverlappedComponent :type "PrimitiveComponent Object Reference") (OtherActor :type "Actor Object Reference") (OtherComp :type "PrimitiveComponent Object Reference") (OtherBodyIndex :type Integer))
  (if (`self.ActorHasTag` OtherActor "Player")
    (`/Game/ContenidoPrincipal/BluePrints/Character/TPC_Principal.HideInteractUI` (`self.PlayerRef`))
    (`SceneComponent.SetVisibility` (`self.Interact Icon`) false false)))

(fn `UserConstructionScript`
  (bind _ns_burststars (`self.NS_BurstStars`))
  (`NiagaraComponent.SetNiagaraVariableLinearColor` (`self.Interact Icon`) "Base Color" (`self.Color Icon`))
  (`FXSystemComponent.SetVectorParameter` _ns_burststars "BoxScale" (60.0 60.0 0.0))
  (`FXSystemComponent.SetVectorParameter` _ns_burststars "Velocity" (0.0 0.0 25.0)))