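; BP_ResiduoNPC is a waste item actor that represents one of five waste categories: plastic, glass, paper, organic or others.
; The construction script calls SetWasteType, which switches on WasteType to assign the matching static mesh, so the look updates in the editor.
; PlaySound switches on the same type to play a category-specific pickup sound at the actor's location; nothing in this Blueprint calls it.
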(event `self.ReceiveBeginPlay`)

(fn `PlaySound`
  (bind _returnvalue (`self.K2_GetActorLocation`))
  (switch `/Game/ContenidoPrincipal/BluePrints/Interfaces/E_WasteType` (`self.WasteType`)
    (:`NewEnumerator0`
      (`GameplayStatics.PlaySoundAtLocation` "/Game/ContenidoPrincipal/Audio/SFX/Plástico_Pickup.Plástico_Pickup" _returnvalue (struct) 1.0 1.0 0.0 null null null))
    (:`NewEnumerator1`
      (`GameplayStatics.PlaySoundAtLocation` "/Game/ContenidoPrincipal/Audio/SFX/Vidrio_Pickup.Vidrio_Pickup" _returnvalue (struct) 1.0 1.0 0.0 null null null))
    (:`NewEnumerator2`
      (`GameplayStatics.PlaySoundAtLocation` "/Game/ContenidoPrincipal/Audio/SFX/Papel_Absorb.Papel_Absorb" _returnvalue (struct) 1.0 1.0 0.0 null null null))
    (:`NewEnumerator3`
      (`GameplayStatics.PlaySoundAtLocation` "/Game/ContenidoPrincipal/Audio/SFX/Grab_02.Grab_02" _returnvalue (struct) 1.0 1.0 0.0 null null null))
    (:`NewEnumerator4`
      (`GameplayStatics.PlaySoundAtLocation` "/Game/ContenidoPrincipal/Audio/SFX/Lata_Pickup.Lata_Pickup" _returnvalue (struct) 1.0 1.0 0.0 null null null))))

(fn `SetWasteType`
  (bind _output_get (set `self.WasteType` (`self.WasteType`)))
  (switch `/Game/ContenidoPrincipal/BluePrints/Interfaces/E_WasteType` _output_get
    (:`NewEnumerator0`
      (`StaticMeshComponent.SetStaticMesh` (`self.MainMesh`) "/Game/ContenidoPrincipal/Meshes/Residuos/Plastics/SM_PlasticBottle.SM_PlasticBottle"))
    (:`NewEnumerator1`
      (`StaticMeshComponent.SetStaticMesh` (`self.MainMesh`) "/Game/ContenidoPrincipal/Meshes/Residuos/Glass/SM_glass_v2.SM_glass_v2"))
    (:`NewEnumerator2`
      (`StaticMeshComponent.SetStaticMesh` (`self.MainMesh`) "/Game/ContenidoPrincipal/Meshes/Residuos/Paper/SM_Paper_1.SM_Paper_1"))
    (:`NewEnumerator3`
      (`StaticMeshComponent.SetStaticMesh` (`self.MainMesh`) "/Game/ContenidoPrincipal/Meshes/Residuos/Organic/SM_Apple.SM_Apple"))
    (:`NewEnumerator4`
      (`StaticMeshComponent.SetStaticMesh` (`self.MainMesh`) "/Game/ContenidoPrincipal/Meshes/Residuos/Others/SM_Can.SM_Can"))))

(fn `UserConstructionScript`
  (`self.SetWasteType`))