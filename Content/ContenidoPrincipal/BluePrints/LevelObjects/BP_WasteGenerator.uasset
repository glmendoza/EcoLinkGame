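; BP_WasteGenerator is a level object that scatters a set Count of interactable BP_Residuo waste actors over an area when play begins.
; The construction script flattens the Area component to the AreaScaleX/Y footprint and tints it with a dynamic material Color.
; SpawnWaste picks random points within the Area bounds, inset horizontally from the edges, and adjusts spawns for collisions.
; It also draws a temporary debug box around the spawn zone.
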(event `self.ReceiveBeginPlay`
  (`self.Spawn Waste`))

(event `Spawn Waste`
  (bind (_origin _boxextent) (`KismetSystemLibrary.GetComponentBounds` (`self.Area`)))
  (bind _returnvalue (- _boxextent (25.0 25.0 0.0)))
  (`KismetSystemLibrary.DrawDebugBox` _origin _returnvalue (struct :`G` 1.0 :`B` 0.833333 :`A` 1.0) (struct) 10.0 2.0)
  (for _ (range (`self.Count`))
    (`|SpawnActorFromClass` "/Game/ContenidoPrincipal/BluePrints/LevelObjects/BP_Residuo.BP_Residuo_C" (`KismetMathLibrary.MakeTransform` (`KismetMathLibrary.RandomPointInBoundingBox` _origin _returnvalue)) "AdjustIfPossibleButAlwaysSpawn" "OverrideRootScale" null "NewEnumerator0" true null)))

(fn `UserConstructionScript`
  (`SceneComponent.SetWorldScale3D` (`self.Area`) (`KismetMathLibrary.MakeVector` (`self.Area Scale X`) (`self.Area Scale Y`) 0.01))
  (bind _returnvalue (`PrimitiveComponent.CreateDynamicMaterialInstance` (`self.Area`) 0 "/Game/ContenidoPrincipal/Materials/Mi_Wall_Color.Mi_Wall_Color" "None"))
  (`MaterialInstanceDynamic.SetVectorParameterValue` _returnvalue "Color" (`self.Color`)))