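; BP_Carteles is an interactable spot where the player places a poster (cartel).
; Its box overlap shows or hides the interact prompt, and Interact reveals the mesh once, triggers a Niagara star burst, increments the GameMode's placed-poster count and refreshes the HUD tab text.
; The construction script applies each instance's CartelTexture through a dynamic material and sets the burst's scale and velocity.
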(event `self.ReceiveBeginPlay`
  (bind _astpc_principal (cast `/Game/ContenidoPrincipal/BluePrints/Character/TPC_Principal` (`GameplayStatics.GetPlayerCharacter` 0)))
  (set `self.PlayerRef` _astpc_principal)
  (bind _astpgame_mode_base (cast `/Game/ContenidoPrincipal/BluePrints/GameModes/TPGameMode_Base` (`GameplayStatics.GetGameMode`)))
  (set `self.GameModeRef` _astpgame_mode_base))

(event `/Game/ContenidoPrincipal/BluePrints/Interfaces/BPI_Interface.Interact`
  (bind _tab (`/Game/ContenidoPrincipal/BluePrints/UI/BP_HUD_Base.Tab` (`/Game/ContenidoPrincipal/BluePrints/Character/TPC_Principal.HUD Ref` (`self.PlayerRef`))))
  (if (not (`SceneComponent.IsVisible` (`self.Cartel`)))
    (`SceneComponent.SetVisibility` (`self.Cartel`) true false)
    (`ActorComponent.Activate` (`self.NS_BurstStars`) false)
    (`/Game/ContenidoPrincipal/BluePrints/Character/TPC_Principal.HideInteractUI` (`self.PlayerRef`))
    (`/Engine/EditorBlueprintResources/StandardMacros.IncrementInt` (`/Game/ContenidoPrincipal/BluePrints/GameModes/TPGameMode_Base.CartelesColocados` (`self.GameModeRef`))
      (:`  `
        (`/Engine/EditorBlueprintResources/StandardMacros.IsValid` _tab
          (:`Is Valid`
            (`/Game/ContenidoPrincipal/BluePrints/UI/Menus/WBP_Tareas.SetTabText` _tab)))))))

(event `self.Box.OnComponentBeginOverlap`
  (params (OverlappedComponent :type "PrimitiveComponent Object Reference") (OtherActor :type "Actor Object Reference") (OtherComp :type "PrimitiveComponent Object Reference") (OtherBodyIndex :type Integer) (bFromSweep :type Boolean) (SweepResult :type "HitResult Structure (by ref)"))
  (if (`self.ActorHasTag` OtherActor "Player")
    (if (not (`SceneComponent.IsVisible` (`self.Cartel`)))
      (`/Game/ContenidoPrincipal/BluePrints/Character/TPC_Principal.ShowInteractUI` (`self.PlayerRef`) "E - Colocar Cartel"))))

(event `self.Box.OnComponentEndOverlap`
  (params (OverlappedComponent :type "PrimitiveComponent Object Reference") (OtherActor :type "Actor Object Reference") (OtherComp :type "PrimitiveComponent Object Reference") (OtherBodyIndex :type Integer))
  (if (`self.ActorHasTag` OtherActor "Player")
    (`/Game/ContenidoPrincipal/BluePrints/Character/TPC_Principal.HideInteractUI` (`self.PlayerRef`))))

(fn `UserConstructionScript`
  (bind _ns_burststars (`self.NS_BurstStars`))
  (bind _returnvalue (`PrimitiveComponent.CreateDynamicMaterialInstance` (`self.Cartel`) 0 "/Game/ContenidoPrincipal/Meshes/Cartel/M_CartelT.M_CartelT" "None"))
  (`MaterialInstanceDynamic.SetTextureParameterValue` _returnvalue "Texture" (`self.CartelTexture`))
  (`FXSystemComponent.SetVectorParameter` _ns_burststars "BoxScale" (0.0 140.0 100.0))
  (`FXSystemComponent.SetVectorParameter` _ns_burststars "Velocity" (5.0 0.0 25.0)))