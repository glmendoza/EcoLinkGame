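; BP_Cigar is a collectible cigar level object that the player picks up as a waste material.
; Its sphere shows or hides an interact prompt on the cached TPC_Principal when a Player-tagged actor overlaps, gated by CanIntereact.
; Interact increments the MaterialsToCollect entry keyed by WasteType and refreshes the cigar HUD.
; The picked cigar is hidden with collision disabled instead of being destroyed.
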(event `/Game/ContenidoPrincipal/BluePrints/Interfaces/BPI_Interface.Interact`
  (if (`self.CanIntereact`)
    (`self.PickCigar`)))

(event `self.ReceiveBeginPlay`
  (bind _astpc_principal (cast `/Game/ContenidoPrincipal/BluePrints/Character/TPC_Principal` (`GameplayStatics.GetPlayerCharacter` 0)))
  (set `self.Player Ref` _astpc_principal))

(event `PickCigar`
  (bind _materialstocollect (`/Game/ContenidoPrincipal/BluePrints/Character/TPC_Principal.MaterialsToCollect` (`self.Player Ref`)))
  (`BlueprintMapLibrary.Map_Add` _materialstocollect (`|GetEnumeratorNameAsString` (`self.WasteType`)) (+ (`BlueprintMapLibrary.Map_Find` _materialstocollect (`|GetEnumeratorNameAsString` (`self.WasteType`))) 1))
  (`self.SetActorEnableCollision` false)
  (`SceneComponent.SetVisibility` (`self.DefaultSceneRoot`) false true)
  (`/Game/ContenidoPrincipal/BluePrints/Character/TPC_Principal.SetCigarHUD` (`self.Player Ref`)))

(event `self.Sphere.OnComponentBeginOverlap`
  (params (OverlappedComponent :type "PrimitiveComponent Object Reference") (OtherActor :type "Actor Object Reference") (OtherComp :type "PrimitiveComponent Object Reference") (OtherBodyIndex :type Integer) (bFromSweep :type Boolean) (SweepResult :type "HitResult Structure (by ref)"))
  (if (`self.ActorHasTag` OtherActor "Player")
    (if (`self.CanIntereact`)
      (`/Game/ContenidoPrincipal/BluePrints/Character/TPC_Principal.ShowInteractUI` (`self.Player Ref`) "E - Recolectar cigarro"))))

(event `self.Sphere.OnComponentEndOverlap`
  (params (OverlappedComponent :type "PrimitiveComponent Object Reference") (OtherActor :type "Actor Object Reference") (OtherComp :type "PrimitiveComponent Object Reference") (OtherBodyIndex :type Integer))
  (if (`self.ActorHasTag` OtherActor "Player")
    (if (`self.CanIntereact`)
      (`/Game/ContenidoPrincipal/BluePrints/Character/TPC_Principal.HideInteractUI` (`self.Player Ref`)))))

(fn `UserConstructionScript`)