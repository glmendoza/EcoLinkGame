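; BP_Residuo is a collectible waste item that randomly becomes plastic, glass, paper, organic or other, with a matching mesh.
; The type is rolled in the Construction Script and re-rolled on BeginPlay, where glass is marked non-interactable.
; For other types, sphere overlap toggles a custom-depth stencil highlight and pickup prompt.
; Interacting increments the player's per-type material count, refreshes the HUD, and hides the item without destroying it.
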(event `self.ReceiveBeginPlay`
  (bind _astpc_principal (cast `/Game/ContenidoPrincipal/BluePrints/Character/TPC_Principal` (`GameplayStatics.GetPlayerCharacter` 0)))
  (set `self.PlayerRef` _astpc_principal)
  (bind _astpgame_mode_base (cast `/Game/ContenidoPrincipal/BluePrints/GameModes/TPGameMode_Base` (`GameplayStatics.GetGameMode`)))
  (set `self.GameModeRef` _astpgame_mode_base)
  (`self.SetWasteType`)
  (set `self.CanInteract` (not (`|EnumEquality` (`self.WasteType`) "NewEnumerator1"))))

(event `/Game/ContenidoPrincipal/BluePrints/Interfaces/BPI_Interface.Interact`
  (if (`self.CanInteract`)
    (`self.PickWaste`)))

(event `PickWaste`
  (bind _materialstocollect (`/Game/ContenidoPrincipal/BluePrints/Character/TPC_Principal.MaterialsToCollect` (`self.PlayerRef`)))
  (`BlueprintMapLibrary.Map_Add` _materialstocollect (`|GetEnumeratorNameAsString` (`self.WasteType`)) (+ (`BlueprintMapLibrary.Map_Find` _materialstocollect (`|GetEnumeratorNameAsString` (`self.WasteType`))) 1))
  (`self.SetActorEnableCollision` false)
  (`SceneComponent.SetVisibility` (`self.MainMesh`) false true)
  (`/Game/ContenidoPrincipal/BluePrints/Character/TPC_Principal.SetMaterialHUD` (`self.PlayerRef`)))

(event `self.SphereColl.OnComponentBeginOverlap`
  (params (OverlappedComponent :type "PrimitiveComponent Object Reference") (OtherActor :type "Actor Object Reference") (OtherComp :type "PrimitiveComponent Object Reference") (OtherBodyIndex :type Integer) (bFromSweep :type Boolean) (SweepResult :type "HitResult Structure (by ref)"))
  (if (`self.ActorHasTag` OtherActor "Player")
    (if (`self.CanInteract`)
      (`PrimitiveComponent.SetCustomDepthStencilValue` (`self.MainMesh`) 3)
      (`/Game/ContenidoPrincipal/BluePrints/Character/TPC_Principal.ShowInteractUI` (`self.PlayerRef`) "E - Recoger"))))

(event `self.SphereColl.OnComponentEndOverlap`
  (params (OverlappedComponent :type "PrimitiveComponent Object Reference") (OtherActor :type "Actor Object Reference") (OtherComp :type "PrimitiveComponent Object Reference") (OtherBodyIndex :type Integer))
  (if (`self.ActorHasTag` OtherActor "Player")
    (if (`self.CanInteract`)
      (`PrimitiveComponent.SetCustomDepthStencilValue` (`self.MainMesh`) 2)
      (`/Game/ContenidoPrincipal/BluePrints/Character/TPC_Principal.HideInteractUI` (`self.PlayerRef`)))))

(fn `SetWasteType`
  (bind _output_get (set `self.WasteType` (cast `/Game/ContenidoPrincipal/BluePrints/Interfaces/E_WasteType` (`KismetMathLibrary.Conv_IntToByte` (`KismetMathLibrary.RandomIntegerInRange` 0 4)))))
  (switch `/Game/ContenidoPrincipal/BluePrints/Interfaces/E_WasteType` _output_get
    (:`NewEnumerator0`
      (`StaticMeshComponent.SetStaticMesh` (`self.MainMesh`) "/Game/ContenidoPrincipal/Meshes/Residuos/Plastics/SM_PlasticBottle.SM_PlasticBottle"))
    (:`NewEnumerator1`
      (`StaticMeshComponent.SetStaticMesh` (`self.MainMesh`) "/Game/ContenidoPrincipal/Meshes/Residuos/Glass/SM_glass_v2.SM_glass_v2"))
    (:`NewEnumerator2`
      (`StaticMeshComponent.SetStaticMesh` (`self.MainMesh`) "/Game/ContenidoPrincipal/Meshes/Residuos/Paper/SM_Paper_1.SM_Paper_1"))
    (:`NewEnumerator3`
      (`StaticMeshComponent.SetStaticMesh` (`self.MainMesh`) "/Game/ContenidoPrincipal/Meshes/Residuos/Organic/SM_Apple.SM_Apple"))
    (:`NewEnumerator4`
      (`StaticMeshComponent.SetStaticMesh` (`self.MainMesh`) "/Game/ContenidoPrincipal/Meshes/Residuos/Others/SM_Can.SM_Can"))))

(fn `UserConstructionScript`
  (`self.SetWasteType`))