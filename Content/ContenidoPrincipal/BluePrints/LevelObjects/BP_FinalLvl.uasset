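; BP_FinalLvl is the level-exit actor, a vehicle the player interacts with to finish the level once it is clean.
; BeginPlay caches the player and game mode, whose LevelClean flag gates both the prompt and the interaction.
; The Box overlap toggles the interact prompt and switches the vehicle's custom-depth stencil as a highlight.
; Interact hides the player HUD, opens WBP_FinalLevelMenu and switches to UI-only input with a visible cursor.
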(event `self.ReceiveBeginPlay`
  (bind _astpc_principal (cast `/Game/ContenidoPrincipal/BluePrints/Character/TPC_Principal` (`GameplayStatics.GetPlayerCharacter` 0)))
  (set `self.Player Ref` _astpc_principal)
  (bind _astpgame_mode_base (cast `/Game/ContenidoPrincipal/BluePrints/GameModes/TPGameMode_Base` (`GameplayStatics.GetGameMode`)))
  (set `self.GameModeRef` _astpgame_mode_base))

(event `/Game/ContenidoPrincipal/BluePrints/Interfaces/BPI_Interface.Interact`
  (bind _returnvalue (`GameplayStatics.GetPlayerController` 0))
  (if (`/Game/ContenidoPrincipal/BluePrints/GameModes/TPGameMode_Base.LevelClean` (`self.GameModeRef`))
    (`Widget.SetRenderOpacity` (`/Game/ContenidoPrincipal/BluePrints/UI/BP_HUD_Base.PlayerHUD Ref` (`/Game/ContenidoPrincipal/BluePrints/Character/TPC_Principal.HUD Ref` (`self.Player Ref`))) 0.0)
    (bind _returnvalue_2 (`|CreateWidget` "/Game/ContenidoPrincipal/BluePrints/UI/Menus/WBP_FinalLevelMenu.WBP_FinalLevelMenu_C" _returnvalue))
    (`UserWidget.AddToViewport` _returnvalue_2 1)
    (set `PlayerController.bShowMouseCursor` true _returnvalue)
    (`WidgetBlueprintLibrary.SetInputMode_UIOnlyEx` _returnvalue null)))

(event `self.Box.OnComponentBeginOverlap`
  (params (OverlappedComponent :type "PrimitiveComponent Object Reference") (OtherActor :type "Actor Object Reference") (OtherComp :type "PrimitiveComponent Object Reference") (OtherBodyIndex :type Integer) (bFromSweep :type Boolean) (SweepResult :type "HitResult Structure (by ref)"))
  (cast `/Game/ContenidoPrincipal/BluePrints/Character/TPC_Principal` OtherActor)
  (if (`/Game/ContenidoPrincipal/BluePrints/GameModes/TPGameMode_Base.LevelClean` (`self.GameModeRef`))
    (`/Game/ContenidoPrincipal/BluePrints/Character/TPC_Principal.ShowInteractUI` (`self.Player Ref`) "E - Finalizar Nivel")
    (`PrimitiveComponent.SetCustomDepthStencilValue` (`self.SM_Vehiculo`) 3)))

(event `self.Box.OnComponentEndOverlap`
  (params (OverlappedComponent :type "PrimitiveComponent Object Reference") (OtherActor :type "Actor Object Reference") (OtherComp :type "PrimitiveComponent Object Reference") (OtherBodyIndex :type Integer))
  (cast `/Game/ContenidoPrincipal/BluePrints/Character/TPC_Principal` OtherActor)
  (`/Game/ContenidoPrincipal/BluePrints/Character/TPC_Principal.HideInteractUI` (`self.Player Ref`))
  (`PrimitiveComponent.SetCustomDepthStencilValue` (`self.SM_Vehiculo`) 2))

(fn `UserConstructionScript`)