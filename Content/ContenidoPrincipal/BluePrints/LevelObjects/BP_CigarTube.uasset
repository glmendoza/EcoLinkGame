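; BP_CigarTube is an interactable deposit point where the player hands in collected waste of its WasteType, with a HUD update for cigars.
; A box overlap by the player toggles the deposit prompt and a Niagara interact icon, tinted in the construction script.
; Interact reports the player's MaterialsToCollect count to the game mode's collected and remaining tallies, zeroes it, then plays a star burst and sound.
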(event `self.ReceiveBeginPlay`
  (bind _astpc_principal (cast `/Game/ContenidoPrincipal/BluePrints/Character/TPC_Principal` (`GameplayStatics.GetPlayerCharacter` 0)))
  (set `self.Player Ref` _astpc_principal)
  (bind _astpgame_mode_base (cast `/Game/ContenidoPrincipal/BluePrints/GameModes/TPGameMode_Base` (`GameplayStatics.GetGameMode`)))
  (set `self.GameModeRef` _astpgame_mode_base))

(event `/Game/ContenidoPrincipal/BluePrints/Interfaces/BPI_Interface.Interact`
  (bind _gamemoderef (`self.GameModeRef`))
  (bind _value (`BlueprintMapLibrary.Map_Find` (`/Game/ContenidoPrincipal/BluePrints/Character/TPC_Principal.MaterialsToCollect` (`self.Player Ref`)) (`|GetEnumeratorNameAsString` (`self.WasteType`))))
  (if (>= _value 1)
    (`/Game/ContenidoPrincipal/BluePrints/GameModes/TPGameMode_Base.WasteRecolected` _gamemoderef _value)
    (`/Game/ContenidoPrincipal/BluePrints/GameModes/TPGameMode_Base.CalculateRemainingWaste` _gamemoderef _value)
    (`BlueprintMapLibrary.Map_Add` (`/Game/ContenidoPrincipal/BluePrints/Character/TPC_Principal.MaterialsToCollect` (`self.Player Ref`)) (`|GetEnumeratorNameAsString` (`self.WasteType`)) (- _value _value))
    (`ActorComponent.Activate` (`self.NS_BurstStars`) true)
    (`GameplayStatics.PlaySoundAtLocation` "/Game/ContenidoPrincipal/Audio/SFX/Tubo.Tubo" (`self.K2_GetActorLocation`) (struct) 1.0 1.0 0.0 null null null)
    (`/Game/ContenidoPrincipal/BluePrints/Character/TPC_Principal.SetCigarHUD` (`self.Player Ref`))))

(event `self.BoxColl.OnComponentBeginOverlap`
  (params (OverlappedComponent :type "PrimitiveComponent Object Reference") (OtherActor :type "Actor Object Reference") (OtherComp :type "PrimitiveComponent Object Reference") (OtherBodyIndex :type Integer) (bFromSweep :type Boolean) (SweepResult :type "HitResult Structure (by ref)"))
  (if (`self.ActorHasTag` OtherActor "Player")
    (`/Game/ContenidoPrincipal/BluePrints/Character/TPC_Principal.ShowInteractUI` (`self.Player Ref`) "E - Depositar Residuos")
    (`SceneComponent.SetVisibility` (`self.Interact Icon`) true false)))

(event `self.BoxColl.OnComponentEndOverlap`
  (params (OverlappedComponent :type "PrimitiveComponent Object Reference") (OtherActor :type "Actor Object Reference") (OtherComp :type "PrimitiveComponent Object Reference") (OtherBodyIndex :type Integer))
  (if (`self.ActorHasTag` OtherActor "Player")
    (`/Game/ContenidoPrincipal/BluePrints/Character/TPC_Principal.HideInteractUI` (`self.Player Ref`))
    (`SceneComponent.SetVisibility` (`self.Interact Icon`) false false)))

(fn `UserConstructionScript`
  (bind _ns_burststars (`self.NS_BurstStars`))
  (`NiagaraComponent.SetNiagaraVariableLinearColor` (`self.Interact Icon`) "Base Color" (`self.Color Icon`))
  (`FXSystemComponent.SetVectorParameter` _ns_burststars "BoxScale" (0.0 10.0 10.0))
  (`FXSystemComponent.SetVectorParameter` _ns_burststars "Velocity" (5.0 0.0 10.0)))